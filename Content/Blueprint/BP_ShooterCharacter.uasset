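; BP_ShooterCharacter is a shooter character that fires its attached item at enemies on left mouse press.
; When it has a weapon, it runs a complex Visibility line trace forward from the capsule, with timed debug drawing.
; Only a hit actor that casts to BP_EnemyPawn is passed to the attached item's Shoot, so misses and other hits do not fire.
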(event Input|MouseEvents|LeftMouseButton
  (params (Key :type Key%20Structure :default "None"))
  (bind _capsulecomponent (Variables|Default|GetCapsuleComponent))
  (bind _returnvalue (Transformation|GetWorldLocation _capsulecomponent))
  (:Pressed
    (if (Variables|Default|GetHasWeapon)
      (bind _outhit (Collision|LineTraceByChannel _returnvalue (+ _returnvalue (* (Math|Vector|GetForwardVector (Transformation|GetWorldRotation _capsulecomponent)) 1e+03)) "TraceTypeQuery1" true 0 "ForDuration"))
      (bind _asbp_enemy_pawn (Utilities|Casting|CastToBP_EnemyPawn (.HitActor (Collision|BreakHitResult _outhit))))
      (Class|WeaponItem|Shoot (Variables|Default|GetAttachedItem) _asbp_enemy_pawn))))

(fn ConstructionScript)