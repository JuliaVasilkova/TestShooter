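; BP_EnemyPawn is an enemy pawn built to chase a sensed TestShooterCharacter and damage it on reaching it.
; PawnSensing feeds AI MoveTo, whose success applies damage, but a constant branch condition keeps this path from running.
; Incoming damage lowers and prints Health unless IsDead, which is never set here.
; The pawn deactivates movement and destroys itself only when Health equals exactly zero.
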(event OnSeePawn(PawnSensing)
  (params (Pawn :type Pawn%20Object%20Reference))
  ;[1 1 1] AI_MoveTo Character logic
  (if (not (not false))
    (bind _astest_shooter_character (Utilities|Casting|CastToTestShooterCharacter Pawn))
    (AI|AIMoveTo self "0, 0, 0" _astest_shooter_character 4e+01 false
      (:OnSuccess
        (Game|Damage|ApplyDamage _astest_shooter_character 1e+01 0 0)))))

(event Game|Damage|EventAnyDamage
  (params (Damage :type Float%20%28single-precision%29) (DamageType :type Damage%20Type%20Object%20Reference) (InstigatedBy :type Controller%20Object%20Reference) (DamageCauser :type Actor%20Object%20Reference))
  (if (not (Variables|Default|GetIsDead))
    (bind _output_get (Variables|Default|SetHealth (- (Variables|Default|GetHealth) Damage)))
    (Development|PrintString (Utilities|String|ToString(Float) _output_get))
    (if (== (Variables|Default|GetHealth) 0.0)
      (Components|Activation|Deactivate (Variables|Default|GetMoveComponent))
      (Actor|DestroyActor))))

(fn ConstructionScript)